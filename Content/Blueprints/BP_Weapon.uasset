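; BP_Weapon is a weapon Blueprint that provides the visual and audio effects of firing.
; Its Fire event spawns the MuzzleFlash effect at the Muzzle component's world transform, then plays FireSound at the actor's location.
; The graph handles no projectile, trace or damage.
; An unused SpawnSystemAttached node, which would attach the flash to WeaponMesh at "Muzzle", remains in the graph but never runs.
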(event `Fire`
  (bind _muzzle (`self.Muzzle`))
  (`NiagaraFunctionLibrary.SpawnSystemAtLocation` (`self.MuzzleFlash`) (`SceneComponent.K2_GetComponentLocation` _muzzle) (`SceneComponent.K2_GetComponentRotation` _muzzle))
  (`GameplayStatics.PlaySoundAtLocation` (`self.Fire Sound`) (`self.K2_GetActorLocation`) (struct) 1.0 1.0 0.0 null null null null))

(fn `UserConstructionScript`)